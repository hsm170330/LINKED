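; BP_B3 is a one-shot button that responds to InteractwithObject and counts toward the Door_Level1Warp door.
; While IsOn is true, pressing it swaps to the red off material, plays a click, moves the cylinder down and clears IsOn.
; It then finds the first RoomComplete3 actor to turn all its static mesh materials green, and increments CurrentCount on the first Door_Level1Warp.
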(event EventInteractwithObject
  (if (Variables|Default|GetIsOn)
    (Rendering|Material|SetMaterial (Variables|Default|GetCylinder) 0 "/Game/Materials/M_Red_Off.M_Red_Off")
    (Audio|PlaySoundatLocation "/Engine/VREditor/Sounds/UI/Click_on_Button_Cue.Click_on_Button_Cue" (Transformation|GetActorLocation) "0, 0, 0" 1.0 1.0 0.0 0 0 0 0)
    (Transformation|SetRelativeLocation (Variables|Default|GetCylinder) "0, 0,-10.000000" false false)
    (Variables|Default|SetIsOn false)
    (bind _outactors (Actor|GetAllActorsOfClass "/Game/BPs/RoomComplete3.RoomComplete3_C"))
    (bind _asactor (Utilities|Casting|CastToActor (Utilities|Array|Get(acopy) _outactors)))
    (for _array_element (Actor|GetComponentsByClass _asactor "/Script/Engine.StaticMeshComponent")
      (for _index (range 0 (- (Rendering|Material|GetNumMaterials _array_element) 1))
        (Rendering|Material|SetMaterial _array_element _index "/Engine/EngineDebugMaterials/VertexColorViewMode_GreenOnly.VertexColorViewMode_GreenOnly")))
    (bind _outactors_2 (Actor|GetAllActorsOfClass "/Game/BPs/Doors/Door_Level1Warp.Door_Level1Warp_C"))
    (bind _asdoor_level_1warp (Utilities|Casting|CastToDoor_Level1Warp (Utilities|Array|Get(acopy) _outactors_2)))
    (Math|Integer|IncrementInt (Variables|/Game/BPs/Doors/Door_Level1Warp.Door_Level1Warp_C|GetCurrentCount _asdoor_level_1warp)
      (:%20%20
        (Development|PrintString "Button Pressed")))))

(fn ConstructionScript
  (|CallParentFunction))