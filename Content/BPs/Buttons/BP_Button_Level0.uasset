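; Level 0 button that, on interaction, activates the level's warp door.
; A press works only while IsOn is true, then clears it, swapping the cylinder to its red off material, lowering it and playing a click.
; It finds the first Door_Level0Warp and paints its static meshes red.
; The door's "Trigger"-tagged mesh turns pure black and gets query and physics collision.
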(event EventInteractwithObject
  (if (Variables|Default|GetIsOn)
    (Rendering|Material|SetMaterial (Variables|Default|GetCylinder) 0 "/Game/Materials/M_Red_Off.M_Red_Off")
    (Audio|PlaySoundatLocation "/Engine/VREditor/Sounds/UI/Click_on_Button_Cue.Click_on_Button_Cue" (Transformation|GetActorLocation) "0, 0, 0" 1.0 1.0 0.0 0 0 0 0)
    (Transformation|SetRelativeLocation (Variables|Default|GetCylinder) "0, 0,-10.000000" false false)
    (Variables|Default|SetIsOn false)
    (bind _outactors (Actor|GetAllActorsOfClass "/Game/BPs/Doors/Door_Level0Warp.Door_Level0Warp_C"))
    (bind _asactor (Utilities|Casting|CastToActor (Utilities|Array|Get(acopy) _outactors)))
    (for _array_element (Actor|GetComponentsByClass _asactor "/Script/Engine.StaticMeshComponent")
      (for _index (range 0 (- (Rendering|Material|GetNumMaterials _array_element) 1))
        (Rendering|Material|SetMaterial _array_element _index "/Game/Materials/M_Red.M_Red")
        (Rendering|Material|SetMaterial (Utilities|Array|Get(acopy) (Actor|GetComponentsbyTag _asactor "/Script/Engine.StaticMeshComponent" "Trigger")) 0 "/Game/SuperGrid/TutorialLevel/MaterialInstances/M_PureBlack.M_PureBlack")
        (Collision|SetCollisionEnabled (Utilities|Array|Get(acopy) (Actor|GetComponentsbyTag _asactor "/Script/Engine.StaticMeshComponent" "Trigger")) "QueryAndPhysics")))))

(fn ConstructionScript
  (|CallParentFunction))