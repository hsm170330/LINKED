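; BP_TimedPlatforms is a platform that briefly disappears after the first-person player touches it.
; Overlap of its Sphere by BP_FirstPersonCharacter darkens the Cylinder's PrimaryColor material parameter as a warning.
; After a short delay both cylinder meshes lose visibility and collision, then after a longer delay they reappear solid with the lighter color set again.
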(event OnComponentBeginOverlap(Sphere)
  (params (OverlappedComponent :type Primitive%20Component%20Object%20Reference) (OtherActor :type Actor%20Object%20Reference) (OtherComp :type Primitive%20Component%20Object%20Reference) (OtherBodyIndex :type Integer) (bFromSweep :type Boolean) (SweepResult :type Hit%20Result%20Structure%20%28by%20ref%29))
  (Utilities|Casting|CastToBP_FirstPersonCharacter OtherActor)
  (Rendering|Material|SetVectorParameterValueonMaterials (Variables|Default|GetCylinder) "PrimaryColor" (Math|Vector|MakeVector 0.003614 0.025728 0.032083))
  (Utilities|FlowControl|Delay 0.75)
  (Rendering|SetVisibility (Variables|Default|GetCylinder) false false)
  (Collision|SetCollisionEnabled (Variables|Default|GetCylinder) "NoCollision")
  (Rendering|SetVisibility (Variables|Default|GetCylinder1) false false)
  (Collision|SetCollisionEnabled (Variables|Default|GetCylinder1) "NoCollision")
  (Utilities|FlowControl|Delay 2.0)
  (Rendering|SetVisibility (Variables|Default|GetCylinder) true false)
  (Collision|SetCollisionEnabled (Variables|Default|GetCylinder) "QueryAndPhysics")
  (Rendering|SetVisibility (Variables|Default|GetCylinder1) true false)
  (Collision|SetCollisionEnabled (Variables|Default|GetCylinder1) "QueryAndPhysics")
  (Rendering|Material|SetVectorParameterValueonMaterials (Variables|Default|GetCylinder) "PrimaryColor" (Math|Vector|MakeVector 0.030457 0.113187 0.165)))

(event EventBeginPlay
  (Input|EnableInput (Game|GetPlayerController 0)))

(fn ConstructionScript)