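; Interactable button that turns floating cubes red when triggered through its InteractwithObject event.
; The event finds BP_FloatingCube actors tagged ChangeColor and sets every material slot on each one's static mesh to red metal.
; The button's own feedback (off material, click sound, lowered cylinder) runs inside the innermost loop, so it repeats per slot and needs a matching cube to fire.
; The cylinder is never reset.
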(event EventInteractwithObject
  (bind _outactors (Actor|GetAllActorsOfClasswithTag "/Game/SuperGrid/TutorialLevel/Blueprints/LevelElements/BP_FloatingCube.BP_FloatingCube_C" "ChangeColor"))
  (for _array_element _outactors
    (for _array_element_2 (Utilities|Array|MakeArray (Actor|GetComponentbyClass _array_element "/Script/Engine.StaticMeshComponent"))
      (for _index (range 0 (- (Rendering|Material|GetNumMaterials _array_element_2) 1))
        (Rendering|Material|SetMaterial _array_element_2 _index "/Game/SuperGrid/TutorialLevel/MaterialInstances/M_Tut_MetalRed.M_Tut_MetalRed")
        (Rendering|Material|SetMaterial (Variables|Default|GetCylinder) 0 "/Game/Materials/M_Red_Off.M_Red_Off")
        (Audio|PlaySoundatLocation "/Engine/VREditor/Sounds/UI/Click_on_Button_Cue.Click_on_Button_Cue" (Transformation|GetActorLocation) "0, 0, 0" 1.0 1.0 0.0 0 0 0 0)
        (Transformation|SetRelativeLocation (Variables|Default|GetCylinder) "0, 0,-10.000000" false false)))))

(fn ConstructionScript
  (|CallParentFunction))