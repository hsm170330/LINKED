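; BP_TurnRed is a trigger actor that turns tagged floating cubes red when anything begins overlapping its TriggerArea.
; The overlap prints the entering actor's name, then gathers every BP_FloatingCube tagged ChangeColor.
; On each cube, it takes a single StaticMeshComponent and replaces every material slot with M_Tut_MetalRed.
; It does not filter the overlapping actor or restore the original materials.
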(event OnComponentBeginOverlap(TriggerArea)
  (params (OverlappedComponent :type Primitive%20Component%20Object%20Reference) (OtherActor :type Actor%20Object%20Reference) (OtherComp :type Primitive%20Component%20Object%20Reference) (OtherBodyIndex :type Integer) (bFromSweep :type Boolean) (SweepResult :type Hit%20Result%20Structure%20%28by%20ref%29))
  (Development|PrintString (Utilities|GetDisplayName OtherActor))
  (bind _outactors (Actor|GetAllActorsOfClasswithTag "/Game/SuperGrid/TutorialLevel/Blueprints/LevelElements/BP_FloatingCube.BP_FloatingCube_C" "ChangeColor"))
  (for _array_element _outactors
    (for _array_element_2 (Utilities|Array|MakeArray (Actor|GetComponentbyClass _array_element "/Script/Engine.StaticMeshComponent"))
      (for _index (range 0 (- (Rendering|Material|GetNumMaterials _array_element_2) 1))
        (Rendering|Material|SetMaterial _array_element_2 _index "/Game/SuperGrid/TutorialLevel/MaterialInstances/M_Tut_MetalRed.M_Tut_MetalRed")))))

(event EventBeginPlay)

(event Collision|EventActorBeginOverlap
  (params (OtherActor :type Actor%20Object%20Reference)))

(event EventTick
  (params (DeltaSeconds :type Float%20%28single-precision%29)))

(fn ConstructionScript)